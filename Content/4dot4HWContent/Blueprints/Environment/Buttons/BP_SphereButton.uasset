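; BP_SphereButton is an environment button labeled "Spheres" that toggles the visibility of interaction spheres when the player overlaps its box.
; On BeginPlay it activates itself and, if MySpheres is empty, fills it with every BP_InteractionSphere in the level.
; A FlipFlop alternates hiding and showing each sphere's static mesh, starting with hide.
; An inactive button only prints a message.
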(event `self.ReceiveBeginPlay`
  (`parent.ReceiveBeginPlay`)
  (`|ExecutionSequence`
    (:`then_0`
      (if (`KismetArrayLibrary.Array_IsEmpty` (`self.MySpheres`))
        (bind _outactors (`GameplayStatics.GetAllActorsOfClass` "/Game/4dot4HWContent/Blueprints/Environment/BP_InteractionSphere.BP_InteractionSphere_C"))
        (bind _output_get (set `self.MySpheres` _outactors))
        (if (`KismetArrayLibrary.Array_IsEmpty` _output_get)
          (`KismetSystemLibrary.PrintString` "There is no Spheres for sphere-button"))))
    (:`then_1`
      (`self.ChangeStateButton` true))
    (:`then_2`
      (`TextRenderComponent.K2_SetText` (`self.TextRender`) "Spheres"))))

(event `/Game/4dot4HWContent/Blueprints/Interfaces/BPI_Switchable.SetVisibleOn`
  (if (`self.IsButtonActive`)
    (for _array_element (`self.MySpheres`)
      (`SceneComponent.SetVisibility` (`/Game/4dot4HWContent/Blueprints/Environment/BP_InteractionSphere.StaticMesh` _array_element) true false))
    (else
      (`KismetSystemLibrary.PrintString` "Sphere-button is not active" true true (struct :`R` 1.0 :`A` 1.0) 5.0 :!label _label))))

(event `/Game/4dot4HWContent/Blueprints/Interfaces/BPI_Switchable.SetVisibleOff`
  (if (`self.IsButtonActive`)
    (for _array_element (`self.MySpheres`)
      (`SceneComponent.SetVisibility` (`/Game/4dot4HWContent/Blueprints/Environment/BP_InteractionSphere.StaticMesh` _array_element) false false))
    (else
      (goto _label))))

(event `self.Box.OnComponentBeginOverlap`
  (params (OverlappedComponent :type "PrimitiveComponent Object Reference") (OtherActor :type "Actor Object Reference") (OtherComp :type "PrimitiveComponent Object Reference") (OtherBodyIndex :type Integer) (bFromSweep :type Boolean) (SweepResult :type "HitResult Structure (by ref)"))
  (if (`GameplayStatics.ObjectIsA` OtherActor (`self.PlayerCharacterClass`))
    (`/Engine/EditorBlueprintResources/StandardMacros.FlipFlop`
      (:`A`
        (`self.SetVisibleOff`))
      (:`B`
        (`self.SetVisibleOn`)))))

(fn `UserConstructionScript`
  (`parent.UserConstructionScript`))
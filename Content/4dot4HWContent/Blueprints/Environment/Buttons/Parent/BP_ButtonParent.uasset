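; BP_ButtonParent is a parent Blueprint for environment buttons that tracks and displays an active or inactive state.
; ChangeStateButton swaps the Plane's material between active and inactive instances and sets the IsButtonActive flag, which a getter function exposes.
; On BeginPlay it caches the player character's class, which nothing else in this Blueprint uses.
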(event `self.ReceiveBeginPlay`
  (set `self.PlayerCharacterClass` (`GameplayStatics.GetObjectClass` (`GameplayStatics.GetPlayerCharacter` 0))))

(fn `ChangeStateButton`
  (params (Active :type Boolean))
  (bind _plane (`self.Plane`))
  (if Active
    (`PrimitiveComponent.SetMaterial` _plane 0 "/Game/4dot4HWContent/Materials/MI_ActiveButton.MI_ActiveButton")
    (set `self.bIsButtonActive` true)
    (else
      (`PrimitiveComponent.SetMaterial` _plane 0 "/Game/4dot4HWContent/Materials/MI_InactiveButton.MI_InactiveButton")
      (set `self.bIsButtonActive` false))))

(fn `IsButtonActive`
  (returns (bIsButtonActive :type Boolean))
  (return (`self.bIsButtonActive`)))

(fn `UserConstructionScript`)
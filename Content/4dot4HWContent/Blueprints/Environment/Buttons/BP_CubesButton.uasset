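; A button Blueprint, labeled "Cubes", that toggles the visibility of interaction cubes when the player character steps into its trigger box.
; On BeginPlay it fills an empty cube list with every BP_InteractionCube in the level and activates itself through ChangeStateButton.
; Box overlaps alternate through a FlipFlop between hiding and showing the cubes' static meshes, starting with hide, and only while the button is active.
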(event `self.ReceiveBeginPlay`
  (`parent.ReceiveBeginPlay`)
  (`|ExecutionSequence`
    (:`then_0`
      (if (`KismetArrayLibrary.Array_IsEmpty` (`self.MyCubes`))
        (bind _outactors (`GameplayStatics.GetAllActorsOfClass` "/Game/4dot4HWContent/Blueprints/Environment/BP_InteractionCube.BP_InteractionCube_C"))
        (bind _output_get (set `self.MyCubes` _outactors))
        (if (`KismetArrayLibrary.Array_IsEmpty` _output_get)
          (`KismetSystemLibrary.PrintString` "There is no Cubes for cube-button"))))
    (:`then_1`
      (`self.ChangeStateButton` true))
    (:`then_2`
      (`TextRenderComponent.K2_SetText` (`self.TextRender`) "Cubes"))))

(event `/Game/4dot4HWContent/Blueprints/Interfaces/BPI_Switchable.SetVisibleOn`
  (if (`self.IsButtonActive`)
    (for _array_element (`self.MyCubes`)
      (`SceneComponent.SetVisibility` (`/Game/4dot4HWContent/Blueprints/Environment/BP_InteractionCube.StaticMesh` _array_element) true false))
    (else
      (`KismetSystemLibrary.PrintString` "Cube-button is not active" true true (struct :`R` 1.0 :`A` 1.0) 5.0 :!label _label))))

(event `/Game/4dot4HWContent/Blueprints/Interfaces/BPI_Switchable.SetVisibleOff`
  (if (`self.IsButtonActive`)
    (for _array_element (`self.MyCubes`)
      (`SceneComponent.SetVisibility` (`/Game/4dot4HWContent/Blueprints/Environment/BP_InteractionCube.StaticMesh` _array_element) false false))
    (else
      (goto _label))))

(event `self.Box.OnComponentBeginOverlap`
  (params (OverlappedComponent :type "PrimitiveComponent Object Reference") (OtherActor :type "Actor Object Reference") (OtherComp :type "PrimitiveComponent Object Reference") (OtherBodyIndex :type Integer) (bFromSweep :type Boolean) (SweepResult :type "HitResult Structure (by ref)"))
  (if (`GameplayStatics.ObjectIsA` OtherActor (`self.PlayerCharacterClass`))
    (`/Engine/EditorBlueprintResources/StandardMacros.FlipFlop`
      (:`A`
        (`self.SetVisibleOff`))
      (:`B`
        (`self.SetVisibleOn`)))))

(fn `UserConstructionScript`
  (`parent.UserConstructionScript`))